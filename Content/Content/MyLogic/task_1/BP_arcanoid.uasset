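; BP_arcanoid is the brick field of an Arkanoid-style game, tracking score as bricks are destroyed.
; The Construction Script builds an X-by-Y grid of static mesh components at set spacing and increments COUNTOFBALLS.
; The Hit event destroys the given component, adds a point and randomly spawns a Dovs or BP_ball actor at the hit location.
; Tick prints the score on screen each frame as debug text.
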(event EventTick
  (params (DeltaSeconds :type Float%20%28single-precision%29))
  (Development|PrintString (Utilities|String|ToString(Integer) (Variables|Default|Getscore)) true true "(R=0.000000,G=0.660000,B=1.000000,A=1.000000)" DeltaSeconds)
  (Development|PrintString "score" true true "(R=0.000000,G=0.660000,B=1.000000,A=1.000000)" DeltaSeconds))

(event Collision|EventHit
  (params (MyComp :type Primitive%20Component%20Object%20Reference) (Other :type Actor%20Object%20Reference) (OtherComp :type Primitive%20Component%20Object%20Reference) (bSelfMoved :type Boolean) (HitLocation :type Vector :default "0, 0, 0") (HitNormal :type Vector :default "0, 0, 0") (NormalImpulse :type Vector :default "0, 0, 0") (Hit :type Hit%20Result%20Structure%20%28by%20ref%29))
  (bind _returnvalue (Math|Transform|MakeTransform HitLocation))
  (Components|DestroyComponent MyComp)
  (Variables|Default|Setscore (+ (Variables|Default|Getscore) 1))
  (if (> (Math|Random|RandomFloatinRange 0.0 5.0) 4.0)
    (Game|SpawnActorfromClass "/Game/MyLogic/task_1/dovs.dovs_C" _returnvalue "Undefined" 0 0)
    (elif (> (Math|Random|RandomFloatinRange 0.0 5.0) 4.0)
      (Game|SpawnActorfromClass "/Game/MyLogic/task_1/BP_ball.BP_ball_C" _returnvalue "Undefined" 0 0))))

(fn ConstructionScript
  (Variables|Default|SetCOUNT_OF_BALLS (+ (Variables|Default|GetCOUNT_OF_BALLS) 1))
  (for _index (range 0 (- (Variables|Default|GetX) 1))
    (for _index_2 (range 0 (- (Variables|Default|GetY) 1))
      (AddComponent|AddStaticMeshComponent false (Math|Transform|MakeTransform (Math|Vector|MakeVector (Math|Conversions|ToFloat(Integer) (* _index (Variables|Default|GetX_Distance))) (Math|Conversions|ToFloat(Integer) (* _index_2 (Variables|Default|GetY_distance))) 0.0))))))